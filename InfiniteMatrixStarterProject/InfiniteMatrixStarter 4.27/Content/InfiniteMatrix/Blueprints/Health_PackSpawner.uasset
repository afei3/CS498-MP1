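; Health pack spawner actor that lays down an initial chain of Health_Pack actors on BeginPlay.
; It first destroys every BP_Tunnel in the level, then spawns the first pack at the player pawn's location when no valid newest pack exists.
; Each following pack spawns at the previous one's SpawnPoint, and every pack receives a reference back to the spawner.
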(event EventBeginPlay
  (CallFunction|SpawnInitialHealthPacks)
  (Development|PrintString "Hello" true true "(R=1.000000,G=0.000000,B=0.007021,A=1.000000)"))

(event Collision|EventActorBeginOverlap
  (params (OtherActor :type Actor%20Object%20Reference)))

(event EventTick
  (params (DeltaSeconds :type Float%20%28single-precision%29)))

(fn ConstructionScript)

(fn SpawnHealthPackatSpawnPoint
  (CallFunction|SpawnHealthPack (Transformation|GetWorldLocation (Variables|/Game/InfiniteMatrix/Blueprints/Health_Pack.Health_Pack_C|GetSpawnPoint (Variables|Default|GetNewestHealthPack)))))

(fn SpawnHealthPack
  (params (SpawnLocation :type Vector))
  (bind _returnvalue (Game|SpawnActorfromClass "/Game/InfiniteMatrix/Blueprints/Health_Pack.Health_Pack_C" (Math|Transform|MakeTransform SpawnLocation "0, 0, 0" "1,1,1") "Undefined" 0 0))
  (bind _output_get (Variables|Default|SetNewestHealthPack _returnvalue))
  (Variables|/Game/InfiniteMatrix/Blueprints/Health_Pack.Health_Pack_C|SetHealthPackSpawner _output_get self))

(fn SpawnInitialHealthPacks
  (Utilities|FlowControl|Sequence
    (:then_0
      (bind _outactors (Actor|GetAllActorsOfClass "/Game/InfiniteMatrix/Blueprints/BP_Tunnel.BP_Tunnel_C"))
      (for _array_element _outactors
        (Actor|DestroyActor _array_element)))
    (:then_1
      (for _index (range 0 2)
        (Utilities|IsValid (Variables|Default|GetNewestHealthPack)
          (:Is%20Valid
            (CallFunction|SpawnHealthPackatSpawnPoint))
          (:Is%20Not%20Valid
            (CallFunction|SpawnHealthPack (Transformation|GetActorLocation (Game|Player|GetPlayerPawn 0)))))))))