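; Health pack pickup actor that disappears when BP_Player enters its trigger zone; no healing is applied here.
; On overlap with EndTriggerZone, it tells HealthPackSpawner to spawn a pack at a spawn point, then destroys itself.
; CreatePack assigns the health pack mesh to HPMesh and rotates it, but nothing in this Blueprint calls it.
; A player hit on the mesh only prints a debug string.
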(event OnComponentBeginOverlap(EndTriggerZone)
  (params (OverlappedComponent :type Primitive%20Component%20Object%20Reference) (OtherActor :type Actor%20Object%20Reference) (OtherComp :type Primitive%20Component%20Object%20Reference) (OtherBodyIndex :type Integer) (bFromSweep :type Boolean) (SweepResult :type Hit%20Result%20Structure%20%28by%20ref%29))
  (Utilities|Casting|CastToBP_Player OtherActor)
  (Default|SpawnHealthPackatSpawnPoint (Variables|Default|GetHealthPackSpawner))
  (Actor|DestroyActor))

(event OnComponentHit(HPMesh)
  (params (HitComponent :type Primitive%20Component%20Object%20Reference) (OtherActor :type Actor%20Object%20Reference) (OtherComp :type Primitive%20Component%20Object%20Reference) (NormalImpulse :type Vector :default "0, 0, 0") (Hit :type Hit%20Result%20Structure%20%28by%20ref%29))
  (Utilities|Casting|CastToBP_Player OtherActor)
  (Development|PrintString "Hello"))

(event EventBeginPlay)

(event Collision|EventActorBeginOverlap
  (params (OtherActor :type Actor%20Object%20Reference)))

(event EventTick
  (params (DeltaSeconds :type Float%20%28single-precision%29)))

(fn ConstructionScript)

(fn CreatePack
  (Components|StaticMesh|SetStaticMesh (Variables|Default|GetHPMesh) "/Game/InfiniteMatrix/Textures/source/Archive/HealthPack.HealthPack")
  (Transformation|AddLocalRotation (Variables|Default|GetHPMesh) (Math|Rotator|MakeRotator 9e+01 9e+01 9e+01) false false))