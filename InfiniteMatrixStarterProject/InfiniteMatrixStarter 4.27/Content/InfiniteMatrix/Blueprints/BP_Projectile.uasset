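; Projectile actor that travels along X until it hits something or its lifetime runs out, scoring a point for the player on non-tunnel hits.
; Tick counts down TimeAlive, moving the actor and additionally offsetting its mesh and, at half rate, its hitbox.
; Mesh overlaps register only below a TimeAlive threshold and skip EndZone-tagged components; hits set a flag that Tick uses to destroy it.
; ShootProjectile assigns the sphere mesh.
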(event OnComponentBeginOverlap(ProjectileMesh)
  (params (OverlappedComponent :type Primitive%20Component%20Object%20Reference) (OtherActor :type Actor%20Object%20Reference) (OtherComp :type Primitive%20Component%20Object%20Reference) (OtherBodyIndex :type Integer) (bFromSweep :type Boolean) (SweepResult :type Hit%20Result%20Structure%20%28by%20ref%29))
  (bind _player (Variables|Default|Getplayer))
  (Math|Float|CompareFloat (Variables|Default|Gettime_alive) 3.0
    (:<
      (if (not (Components|ComponentHasTag OtherComp "EndZone"))
        (Utilities|Casting|CastToBP_Tunnel OtherActor
          (:then
            (Variables|Default|Sethit true))
          (:CastFailed
            (bind _result (Math|Integer|IncrementInt (Variables|/Game/InfiniteMatrix/Blueprints/BP_Player.BP_Player_C|GetScore _player))
              (:%20%20
                (Variables|/Game/InfiniteMatrix/Blueprints/BP_Player.BP_Player_C|SetScore _player _result)
                (Variables|Default|Sethit true)))))))))

(event EventBeginPlay)

(event Collision|EventActorBeginOverlap
  (params (OtherActor :type Actor%20Object%20Reference)))

(event EventTick
  (params (DeltaSeconds :type Float%20%28single-precision%29))
  (bind _move_speed (Variables|Default|Getmove_speed))
  (bind _returnvalue (* DeltaSeconds _move_speed))
  (if (Variables|Default|Gethit)
    (Actor|DestroyActor :!label _label)
    (else
      (bind _output_get (Variables|Default|Settime_alive (- (Variables|Default|Gettime_alive) DeltaSeconds)))
      (Math|Float|CompareFloat _output_get 0.0
        (:>
          (Transformation|AddActorWorldOffset (Math|Vector|MakeVector _returnvalue 0.0 0.0))
          (Transformation|AddLocalOffset (Variables|Default|GetProjectileMesh) (Math|Vector|MakeVector _returnvalue 0.0 0.0) false false)
          (Transformation|AddLocalOffset (Variables|Default|GetProjectileHitbox) (Math|Vector|MakeVector (* _returnvalue 0.5) 0.0 0.0) false false))
        (:==
          (goto _label))
        (:<
          (goto _label))))))

(fn ConstructionScript)

(fn ShootProjectile
  (Components|StaticMesh|SetStaticMesh (Variables|Default|GetProjectileMesh) "/Game/InfiniteMatrix/Blueprints/Sphere.Sphere"))