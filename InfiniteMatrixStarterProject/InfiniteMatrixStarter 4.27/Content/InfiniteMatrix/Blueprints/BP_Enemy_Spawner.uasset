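; Enemy spawner that replaces any BP_Enemy actors already in the level with a short initial chain of new ones on BeginPlay.
; Without a valid NewestEnemy it spawns at the player pawn's location; otherwise it uses that enemy's EnemySpawnPoint, so each spawn extends from the previous one.
; Each new enemy becomes NewestEnemy, receives a reference back to the spawner and is initialized through CreateEnemy.
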(event EventBeginPlay
  (CallFunction|SpawnInitialEnemies))

(event Collision|EventActorBeginOverlap
  (params (OtherActor :type Actor%20Object%20Reference)))

(event EventTick
  (params (DeltaSeconds :type Float%20%28single-precision%29)))

(fn ConstructionScript)

(fn SpawnInitialEnemies
  (Utilities|FlowControl|Sequence
    (:then_0
      (bind _outactors (Actor|GetAllActorsOfClass "/Game/InfiniteMatrix/Blueprints/BP_Enemy.BP_Enemy_C"))
      (for _array_element _outactors
        (Actor|DestroyActor _array_element)))
    (:then_1
      (for _index (range 0 2)
        (Utilities|IsValid (Variables|Default|GetNewestEnemy)
          (:Is%20Valid
            (CallFunction|SpawnEnemyatSpawnPoint))
          (:Is%20Not%20Valid
            (CallFunction|SpawnEnemy (Transformation|GetActorLocation (Game|Player|GetPlayerPawn 0)))))))))

(fn SpawnEnemy
  (params (SpawnLocation :type Vector))
  (bind _returnvalue (Game|SpawnActorfromClass "/Game/InfiniteMatrix/Blueprints/BP_Enemy.BP_Enemy_C" (Math|Transform|MakeTransform SpawnLocation "0, 0, 0" "1,1,1") "Undefined" 0 0))
  (bind _output_get (Variables|Default|SetNewestEnemy _returnvalue))
  (Variables|/Game/InfiniteMatrix/Blueprints/BP_Enemy.BP_Enemy_C|SetEnemySpawner _output_get self)
  (Default|CreateEnemy _output_get))

(fn SpawnEnemyatSpawnPoint
  (CallFunction|SpawnEnemy (Transformation|GetWorldLocation (Variables|/Game/InfiniteMatrix/Blueprints/BP_Enemy.BP_Enemy_C|GetEnemySpawnPoint (Variables|Default|GetNewestEnemy)))))