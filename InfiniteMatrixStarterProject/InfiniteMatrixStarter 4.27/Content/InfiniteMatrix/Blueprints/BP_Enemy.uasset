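; Enemy obstacle that costs the player one Health on hit, with a camera shake, and triggers death and the restart display at zero or below.
; A non-fatal hit, a projectile hit or the player reaching the end trigger makes EnemySpawner spawn at a spawn point, then destroys this actor.
; CreateEnemy assigns the HealthPack mesh and applies one randomized local offset to both mesh and hitbox.
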(event OnComponentBeginOverlap(EnemyHitBox)
  (params (OverlappedComponent :type Primitive%20Component%20Object%20Reference) (OtherActor :type Actor%20Object%20Reference) (OtherComp :type Primitive%20Component%20Object%20Reference) (OtherBodyIndex :type Integer) (bFromSweep :type Boolean) (SweepResult :type Hit%20Result%20Structure%20%28by%20ref%29))
  (bind _asbp_player (Utilities|Casting|CastToBP_Player OtherActor)
    (:then
      (Class|MatineeCameraShake|StartMatineeCameraShake (Game|GetPlayerCameraManager 0) "/Game/InfiniteMatrix/Blueprints/Camera_Shake.Camera_Shake_C" 1.0 "UserDefined" "0.000000,0.000000,0.000000")
      (bind _result (Math|Integer|DecrementInt (Variables|/Game/InfiniteMatrix/Blueprints/BP_Player.BP_Player_C|GetHealth _asbp_player))
        (:%20%20
          (bind _output_get (Variables|/Game/InfiniteMatrix/Blueprints/BP_Player.BP_Player_C|SetHealth _asbp_player _result))
          (Math|Integer|CompareInt _output_get
            (:>
              (Default|SpawnEnemyatSpawnPoint (Variables|Default|GetEnemySpawner) :!label _label)
              (Actor|DestroyActor))
            (:==
              (Variables|/Game/InfiniteMatrix/Blueprints/BP_Player.BP_Player_C|SetIs_dead _asbp_player true :!label _label_2)
              (if true
                (Default|DisplayRestart _asbp_player)
                (else
                  (goto _label))))
            (:<
              (goto _label_2))))))
    (:CastFailed
      (Utilities|Casting|CastToBP_Projectile OtherActor)
      (goto _label))))

(event OnComponentBeginOverlap(EndTriggerZone)
  (params (OverlappedComponent :type Primitive%20Component%20Object%20Reference) (OtherActor :type Actor%20Object%20Reference) (OtherComp :type Primitive%20Component%20Object%20Reference) (OtherBodyIndex :type Integer) (bFromSweep :type Boolean) (SweepResult :type Hit%20Result%20Structure%20%28by%20ref%29))
  (Utilities|Casting|CastToBP_Player OtherActor)
  (Default|SpawnEnemyatSpawnPoint (Variables|Default|GetEnemySpawner))
  (Actor|DestroyActor))

(event EventBeginPlay)

(event Collision|EventActorBeginOverlap
  (params (OtherActor :type Actor%20Object%20Reference)))

(event EventTick
  (params (DeltaSeconds :type Float%20%28single-precision%29)))

(fn ConstructionScript)

(fn CreateEnemy
  (Components|StaticMesh|SetStaticMesh (Variables|Default|GetEnemyMesh) "/Game/InfiniteMatrix/Textures/source/Archive/HealthPack.HealthPack")
  (bind _output_get (Variables|Default|Setdx (Math|Random|RandomFloatinRange 0.0 5e+02)))
  (bind _output_get_2 (Variables|Default|Setdy (Math|Random|RandomFloatinRange -1e+02 1e+02)))
  (bind _output_get_3 (Variables|Default|Setdz (Math|Random|RandomFloatinRange 1e+02 1e+02)))
  (Transformation|AddLocalOffset (Variables|Default|GetEnemyMesh) (Math|Vector|MakeVector _output_get _output_get_2 _output_get_3) false false)
  (Transformation|AddLocalOffset (Variables|Default|GetEnemyHitBox) (Math|Vector|MakeVector _output_get _output_get_2 _output_get_3) false false))